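; Obstacle spawner actor for the shooting arcade game that periodically creates asteroids or health pickups at its own transform.
; BeginPlay starts a timer with a random delay between the minimum and maximum spawn times.
; Each Spawn call rolls against a pickup probability to choose a Health_Pickup or an Asteroid, then re-arms the timer with a new random delay, forming an endless irregular spawn loop.
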(event `self.ReceiveBeginPlay`
  (`KismetSystemLibrary.K2_SetTimer` null "Spawn" (`KismetMathLibrary.RandomFloatInRange` (`self.SpawnTimeMin`) (`self.SpawnTimeMax`))))

(fn `Spawn`
  (if (< (`KismetMathLibrary.RandomFloat`) (`self.HealthPickupProbability`))
    (`|SpawnActorFromClass` "/Game/ShootingArcade/Blueprints/Health_Pickup.Health_Pickup_C" (`self.GetTransform`) "Undefined" "OverrideRootScale" null null)
    (else
      (`|SpawnActorFromClass` "/Game/ShootingArcade/Blueprints/Asteroid.Asteroid_C" (`self.GetTransform`) "Undefined" "OverrideRootScale" null null)))
  (`KismetSystemLibrary.K2_SetTimer` null "Spawn" (`KismetMathLibrary.RandomFloatInRange` (`self.SpawnTimeMin`) (`self.SpawnTimeMax`))))

(fn `UserConstructionScript`)