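; Player spaceship for an arcade shooter, moved sideways by the MoveRight axis.
; Holding Bang sets a Shooting flag, and a Delay on Tick throttles the repeated spawning of Plasma_Bolt at the ship's transform.
; A first TakeDamage call turns on damage particles, which HealDamage clears, while a second triggers OnDeath.
; OnDeath spawns an explosion, hides the ship, disables collision and sets a timer for the GameMode's RestartGame.
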(event `InputAxis|MoveRight`
  (params (AxisValue :type "Float (single-precision)"))
  ;[1 1 1] 우측 이동
  (`self.AddMovementInput` (`KismetMathLibrary.GetRightVector` (struct)) AxisValue))

(event `InputAction|Bang`
  (params (Key :type "Key Structure"))
  (:`Pressed`
    (set `self.Shooting` true))
  (:`Released`
    (set `self.Shooting` false)))

(event `self.ReceiveTick`
  (params (DeltaSeconds :type "Float (single-precision)"))
  (`KismetSystemLibrary.Delay` 0.2)
  (if (`self.Shooting`)
    (`|SpawnActorFromClass` "/Game/ShootingArcade/Blueprints/Plasma_Bolt.Plasma_Bolt_C" (`self.GetTransform`) "Undefined" "OverrideRootScale" null null)))

(event `self.ReceiveBeginPlay`)

(fn `HealDamage`
  (set `self.IsDamaged` false)
  (`ActorComponent.Deactivate` (`self.DamageParticleSystem`)))

(fn `OnDeath`
  (`GameplayStatics.SpawnEmitterAtLocation` "/Game/StarterContent/Particles/P_Explosion.P_Explosion" (`self.K2_GetActorLocation`))
  (`self.SetActorHiddenInGame` true)
  (`self.SetActorEnableCollision` false)
  (`KismetSystemLibrary.K2_SetTimer` (`GameplayStatics.GetGameMode`) "RestartGame" 3.0))

(fn `TakeDamage`
  (if (`self.IsDamaged`)
    (`self.OnDeath`)
    (else
      (set `self.IsDamaged` true)
      (`ActorComponent.Activate` (`self.DamageParticleSystem`) false))))

(fn `UserConstructionScript`)